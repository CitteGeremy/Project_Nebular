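; BP_BaseItem is a base item Blueprint for world pickups that characters collect by interacting with them.
; On Interaction, it checks the character's inventory for space, passes its ItemInfo struct through PickUpMessage, then destroys itself; with no space, nothing happens.
; The Construction Script writes the actor's own class into ItemInfo, keeping the other fields, so the item data records which class it came from.
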(event EventBeginPlay
  (|CallParentFunction) ; This node is disabled and will not be called.\nDrag off pins to build functionality.
)

(event Collision|EventActorBeginOverlap
  (params (OtherActor :type Actor%20Object%20Reference))
  (|CallParentFunction OtherActor) ; This node is disabled and will not be called.\nDrag off pins to build functionality.
)

(event EventTick
  (params (DeltaSeconds :type Float%20%28single-precision%29))
  (|CallParentFunction DeltaSeconds) ; This node is disabled and will not be called.\nDrag off pins to build functionality.
)

(event EventInteraction
  (params (Character :type BP%20Third%20Person%20Character%20Object%20Reference))
  (if (Default|HasSpaceinInventory Character)
    (Class|BPIInteract|PickUp(Message) Character (Variables|Default|GetItemInfo))
    (Actor|DestroyActor)))

(fn ConstructionScript
  (Variables|Default|SetItemInfo (Utilities|Struct|MakeS_ItemInfos (.itemtype (Variables|Default|GetItemInfo)) (.itemname (Variables|Default|GetItemInfo)) (.itemdescription (Variables|Default|GetItemInfo)) (.itemicon (Variables|Default|GetItemInfo)) (Utilities|GetClass self) (.itemindex (Variables|Default|GetItemInfo))))
  (|CallParentFunction))