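; BP_BaseInteract is a base actor for interactable objects, with a mesh and a sphere trigger.
; When BP_ThirdPersonCharacter enters or leaves the trigger, it registers or unregisters the object as an interactable with that character.
; The construction script applies configurable mesh scale and trigger radius, and SetOutline toggles custom depth rendering on the mesh for highlighting.
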(event OnComponentBeginOverlap(TriggerInteract)
  (params (OverlappedComponent :type Primitive%20Component%20Object%20Reference) (OtherActor :type Actor%20Object%20Reference) (OtherComp :type Primitive%20Component%20Object%20Reference) (OtherBodyIndex :type Integer) (bFromSweep :type Boolean) (SweepResult :type Hit%20Result%20Structure%20%28by%20ref%29))
  (bind _asbp_third_person_character (Utilities|Casting|CastToBP_ThirdPersonCharacter OtherActor))
  (Class|BPIInteract|RegisterInteractable(Message) _asbp_third_person_character self))

(event OnComponentEndOverlap(TriggerInteract)
  (params (OverlappedComponent :type Primitive%20Component%20Object%20Reference) (OtherActor :type Actor%20Object%20Reference) (OtherComp :type Primitive%20Component%20Object%20Reference) (OtherBodyIndex :type Integer))
  (bind _asbp_third_person_character (Utilities|Casting|CastToBP_ThirdPersonCharacter OtherActor))
  (Class|BPIInteract|UnRegisterInteractable(Message) _asbp_third_person_character self))

(event EventBeginPlay)

(event Collision|EventActorBeginOverlap
  (params (OtherActor :type Actor%20Object%20Reference)))

(event EventTick
  (params (DeltaSeconds :type Float%20%28single-precision%29)))

(fn ConstructionScript
  (Transformation|SetWorldScale3D (Variables|Default|GetSM_Item) (Variables|Size|GetMeshScale))
  (Components|Sphere|SetSphereRadius (Variables|Default|GetTriggerInteract) (Variables|Size|GetSphereTriggerSize) true))

(fn SetOutline
  (params (Outline? :type Boolean))
  (Rendering|SetRenderCustomDepth (Variables|Default|GetSM_Item) Outline?))