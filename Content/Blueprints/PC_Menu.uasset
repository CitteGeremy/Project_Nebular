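; PC_Menu is a menu controller that puts the main menu widget on screen and handles a key to close an overlay.
; On BeginPlay it adds MenuWidget to the viewport and creates a WB_SVideos widget, stored without being displayed.
; Pressing P while VideoOpen is set removes all top-level WB_Settings widgets and clears the flag.
; The file never sets VideoOpen true, and an unconnected WBSettings removal chain never runs.
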(event EventBeginPlay
  (bind _returnvalue (UserInterface|CreateWidget (Variables|Default|GetMenuWidget)))
  (UserInterface|Viewport|AddtoViewport _returnvalue 0)
  (bind _returnvalue_2 (UserInterface|CreateWidget "/Game/UI/PauseMenu/WB_SVideos.WB_SVideos_C"))
  (Variables|Default|SetWB_Videos _returnvalue_2))

(event EventTick
  (params (DeltaSeconds :type Float%20%28single-precision%29)))

(event Input|KeyboardEvents|P
  (params (Key :type Key%20Structure))
  (:Pressed
    (if (Variables|Default|GetVideoOpen?)
      (bind _foundwidgets (Widget|GetAllWidgetsOfClass "/Game/UI/PauseMenu/WB_Settings.WB_Settings_C" true))
      (for _array_element _foundwidgets
        (Widget|RemovefromParent _array_element)
        (Variables|Default|SetVideoOpen? false)))))

(fn ConstructionScript)